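; Player Blueprint for a tactical RPG that provides a zoomable spring arm camera.
; BeginPlay sets the starting arm length to half the maximum zoom and derives a pitch threshold from the minimum zoom.
; The CameraZoom axis event adjusts a clamped target length and eases the arm toward it with FInterpTo.
; Arm pitch eases between two angles depending on whether the target length falls below that threshold.
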(event EventBeginPlay
  (CallFunction|InitCamera))

(event Input|AxisEvents|InputAxisCameraZoom
  (params (AxisValue :type Float%20%28single-precision%29))
  (CallFunction|Zoom AxisValue))

(fn ConstructionScript)

(fn Zoom
  (params (Axis :type Float%20%28single-precision%29))
  (bind _output_get (Variables|Zoom|SetDesiredCameraLenght (Math|Float|Clamp(Float) (+ (* Axis (Variables|Zoom|GetZoomSpeed)) (Variables|Zoom|GetDesiredCameraLenght)) (Variables|Zoom|GetZoomMin) (Variables|Zoom|GetZoomMax))))
  (Variables|/Script/Engine.SpringArmComponent|SetTargetArmLength (Variables|Default|GetSpringArm) (Math|Interpolation|FInterpTo (Variables|/Script/Engine.SpringArmComponent|GetTargetArmLength (Variables|Default|GetSpringArm)) _output_get (Utilities|Time|GetWorldDeltaSeconds) 8.0))
  (if (< (Variables|Zoom|GetDesiredCameraLenght) (Variables|Zoom|GetCameraPitchThresold))
    (CallFunction|SetCameraPitch (Variables|Zoom|GetCameraPitchMin))
    (else
      (CallFunction|SetCameraPitch (Variables|Zoom|GetCameraPitchMax)))))

(fn InitCamera
  (bind _output_get (Variables|/Script/Engine.SpringArmComponent|SetTargetArmLength (Variables|Default|GetSpringArm) (/ (Variables|Zoom|GetZoomMax) 2.0)))
  (Variables|Zoom|SetDesiredCameraLenght _output_get)
  (Variables|Zoom|SetCameraPitchThresold (+ (/ (Variables|Zoom|GetZoomMin) 4.0) (Variables|Zoom|GetZoomMin))))

(fn SetCameraPitch
  (params (DesiredAngle :type Float%20%28single-precision%29))
  (Transformation|SetRelativeRotation (Variables|Default|GetSpringArm) (Math|Rotator|MakeRotator 0.0 (Math|Interpolation|FInterpTo (.pitch (Variables|/Script/Engine.SceneComponent|GetRelativeRotation (Variables|Default|GetSpringArm))) DesiredAngle (Utilities|Time|GetWorldDeltaSeconds) 8.0) 0.0) false false))